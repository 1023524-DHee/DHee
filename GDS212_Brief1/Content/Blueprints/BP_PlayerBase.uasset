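; Base player for a sprite-based game where gravity rotates in 90-degree steps around four directions.
; Q and E cycle the direction ID, but only while grounded.
; Each tick maps that ID to gravity, movement axis and sprite rotation, and drives capsule velocity along gravity at constant fall speed.
; A short line trace along gravity detects ground and stops the fall, while MoveRight input moves along the rotated axis.
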(event EventBeginPlay)

(event EventTick
  (params (DeltaSeconds :type Float%20%28single-precision%29))
  (bind _capsulecomponent (Variables|Collision|GetCapsuleComponent))
  (bind _returnvalue (Transformation|GetWorldLocation _capsulecomponent))
  ;[1 1 1] Update Current Gravity
  (Physics|SetPhysicsLinearVelocity (Variables|Collision|GetCapsuleComponent) (* (Variables|Default|GetGravityDirection) (Variables|Default|GetFallSpeed)) false "None")
  ;[1 1 1] Set Gravity & Rotation on KeyPress
  (switch int (Variables|Default|GetDirectionID)
    (:0
      (Variables|Default|SetFallSpeed 6e+02)
      (Variables|Default|SetMovementDirection "1.000000, 0, 0")
      (Variables|Default|SetGravityDirection "0.000000,0.000000,-1.000000")
      (Transformation|SetWorldRotation (Variables|Default|GetSprite) "0, 0, 0" false false))
    (:1
      (Variables|Default|SetFallSpeed 6e+02)
      (Variables|Default|SetMovementDirection "0, 0,1.000000")
      (Variables|Default|SetGravityDirection "1.000000, 0,0.000000")
      (Transformation|SetWorldRotation (Variables|Default|GetSprite) "90.000000, 0, 0" false false))
    (:2
      (Variables|Default|SetFallSpeed 6e+02)
      (Variables|Default|SetMovementDirection "-1.000000, 0, 0")
      (Variables|Default|SetGravityDirection "0.000000,0.000000,1.000000")
      (Transformation|SetWorldRotation (Variables|Default|GetSprite) "180.000000, 0, 0" false false))
    (:3
      (Variables|Default|SetFallSpeed 6e+02)
      (Variables|Default|SetMovementDirection "0, 0,-1.000000")
      (Variables|Default|SetGravityDirection "-1.000000, 0,0.000000")
      (Transformation|SetWorldRotation (Variables|Default|GetSprite) "-90.000000, 0, 0" false false)))
  ;[1 1 1] Detect Ground
  (bind _returnvalue_2 (Collision|LineTraceByChannel _returnvalue (+ _returnvalue (* (Variables|Default|GetGravityDirection) 5e+01)) "TraceTypeQuery1" false 0 "None"))
  (if _returnvalue_2
    (Variables|Default|SetFallSpeed 0.0)
    (Variables|Default|SetTouchedGround true)
    (else
      (Variables|Default|SetFallSpeed 6e+02)
      (Variables|Default|SetTouchedGround false))))

(event Input|AxisEvents|InputAxisMoveRight
  (params (AxisValue :type Float%20%28single-precision%29))
  ;[1 1 1] Update Player LR Movement
  (Pawn|Input|AddMovementInput (Variables|Default|GetMovementDirection) AxisValue false))

(event Input|KeyboardEvents|Q
  (params (Key :type Key%20Structure :default "None"))
  ;[1 1 1] Rotation Input
  (:Pressed
    (if (Variables|Default|GetTouchedGround)
      (Variables|Default|SetDirectionID (Math|Integer|%(Integer) (+ (Variables|Default|GetDirectionID) 1) 4)))))

(event Input|KeyboardEvents|E
  (params (Key :type Key%20Structure :default "None"))
  ;[1 1 1] Rotation Input
  (:Pressed
    (if (Variables|Default|GetTouchedGround)
      (if (== (Variables|Default|GetDirectionID) 0)
        (Variables|Default|SetDirectionID 3)
        (else
          (Variables|Default|SetDirectionID (- (Variables|Default|GetDirectionID) 1)))))))

(fn ConstructionScript)